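; Player controller that creates the player's HUD and keeps it updated with online subsystem status from the game mode.
; On BeginPlay it adds a WBP_Hud widget to the player screen and caches BP_GameMode, printing an error if the cast fails.
; Every Tick it copies the current subsystem and whether the Epic subsystem is loaded from the game mode into the HUD, without validity checks.
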(event `self.ReceiveBeginPlay`
  (bind _returnvalue (`|CreateWidget` "/Game/UI/WBP_Hud.WBP_Hud_C" self))
  (bind _output_get (set `self.HUDWidget` _returnvalue))
  (`UserWidget.AddToPlayerScreen` _output_get 0)
  (bind _asbp_game_mode (cast `/Game/Blueprints/BP_GameMode` (`GameplayStatics.GetGameMode`))
    (:`then`
      (set `self.BPGameMode` _asbp_game_mode))
    (:`CastFailed`
      (`KismetSystemLibrary.PrintString` "PlayerController could not cast to bp game mode" true true (struct :`R` 1.0 :`B` 0.057555 :`A` 1.0) 20.0))))

(event `self.ReceiveTick`
  (params (DeltaSeconds :type "Float (single-precision)"))
  (set `/Game/UI/WBP_Hud.CurrentSubsystem` (`EOSDemoGameModeBase.GetCurrentSubsystem` (`self.BPGameMode`)) (`self.HUDWidget`))
  (set `/Game/UI/WBP_Hud.isEpicSubsystemLoaded?` (`EOSDemoGameModeBase.IsEpicSubsystemLoaded` (`self.BPGameMode`)) (`self.HUDWidget`)))

(fn `UserConstructionScript`)